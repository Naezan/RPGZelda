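; Game mode for an RPG that controls player spawning and relays save and load requests.
; New players restart at the PlayerStart found by name, using the options string minus its first character, so level travel can pick the spawn.
; The ChoosePlayerStart override prefers the start tagged Town_Start.
; SaveGame and LoadGame forward to the RPG game instance cached on BeginPlay and print a debug message.
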(event Custom|SaveGame
  (Class|RPGGameInstance|WriteSaveGame (Variables|Default|GetRPGGame%20Instance))
  (Development|PrintString "SaveGame"))

(event Custom|LoadGame
  (params (NewParam :type Player%20Controller%20Object%20Reference))
  (Class|RPGGameInstance|LoadSaveGame (Variables|Default|GetRPGGame%20Instance) NewParam)
  (Development|PrintString "LoadGame"))

(event EventBeginPlay
  (bind _asbp_rpggame_instance (Utilities|Casting|CastToBP_RPGGameInstance (Game|GetGameInstance)))
  (Variables|Default|SetRPGGame%20Instance _asbp_rpggame_instance))

(event EventTick
  (params (DeltaSeconds :type Float%20%28single-precision%29)))

(event EventHandleStartingNewPlayer
  (params (NewPlayer :type Player%20Controller%20Object%20Reference))
  (bind _optionsstring (Variables|Default|GetOptionsString))
  (Class|GameModeBase|RestartPlayeratPlayerStart NewPlayer (Class|GameModeBase|FindPlayerStart NewPlayer (Utilities|String|GetSubstring _optionsstring 1 (- (Utilities|String|Len _optionsstring) 1)))))

(fn ConstructionScript)

(fn ChoosePlayerStart
  (params (Player :type Controller%20Object%20Reference))
  (bind _outactors (Actor|GetAllActorsOfClass "/Script/Engine.PlayerStart"))
  (for _array_element _outactors
    (Utilities|IsValid _array_element
      (:Is%20Valid
        (if (Utilities|Name|Equal(Name) (Variables|/Script/Engine.PlayerStart|GetPlayerStartTag _array_element) "Town_Start")
          (return _array_element)))))
  (return _array_element))