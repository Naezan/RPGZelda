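; BP_BlaazSplitCharacter is a split clone of the Blaaz character, showing its index number on a widget.
; On BeginPlay it runs a timeline that calls MoveToStartPoint each update along its Forward value, then restores walking and the Pawn collision profile.
; StopMoveCharacter disables movement once and ignores Pawn collision so clones do not block each other, until ResetMovement reverses it.
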(event Custom|SelfSplit
  (Timeline|MoveToPoint Play ; 다른액터에서 호출하면 타임라인 재생안됨 왜이런지 모르겠음
    (:Update
      (Class|BlaazSplitCharacter|MovetoStartPoint (Variables|Default|GetForward) (Utilities|Time|GetWorldDeltaSeconds)))
    (:Finished
      (CallFunction|ResetMovement))))

(event EventBeginPlay
  (CallFunction|SelfSplit) ; 시작할때 분신끼리의 충돌막기
  (bind _aswbp_split_index (Utilities|Casting|CastToWBP_SplitIndex (UserInterface|GetWidget (Variables|Default|GetNumberWidget))))
  (Rendering|Components|TextRender|SetText (Variables|/Game/UI/WBP_SplitIndex.WBP_SplitIndex_C|GetIndexText _aswbp_split_index) (Utilities|Text|ToText(Integer) (Variables|Default|GetIndex))))

(event EventResetMovement
  (bind _capsulecomponent (Variables|Default|GetCapsuleComponent))
  (Variables|Default|SetbStopMoving false)
  (Collision|SetCollisionProfileName _capsulecomponent "Pawn" true :!class /Script/Engine.PrimitiveComponent)
  (Collision|SetCollisionResponsetoChannel _capsulecomponent "ECC_Visibility" "ECR_Block")
  (Pawn|Components|CharacterMovement|SetMovementMode (Variables|Character|GetCharacterMovement) "MOVE_Walking" 0))

(event EventStopMoveCharacter
  (if (not (Variables|Default|GetbStopMoving))
    (Variables|Default|SetbStopMoving true)
    (Pawn|Components|CharacterMovement|DisableMovement (Variables|Character|GetCharacterMovement))
    (Collision|SetCollisionResponsetoChannel (Variables|Default|GetCapsuleComponent) "ECC_Pawn" "ECR_Ignore") ; 서로 충돌되는것을 막기
    (Development|PrintString "오브젝트 위치에 파티클")))

(fn ConstructionScript)