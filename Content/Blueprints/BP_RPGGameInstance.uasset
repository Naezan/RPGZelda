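; BP_RPGGameInstance is the RPG's game instance Blueprint, handling item preloading and level load transitions.
; InitItems async-loads the primary assets for each type key in ItemsPerType and adds those that cast to RPGItem to StoreItems.
; LoadGameLevel clears widgets, shows a loading screen and opens a level whose name is unset; RestartGameLevel reuses it.
; Init is empty, leaving its LoadSaveGame and InitItems calls disconnected.
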(event Custom|LoadGameLevel
  (Viewport|RemoveAllWidgets)
  (Class|RPGBlueprintLibrary|PlayLoadingScreen true 3.0)
  (Game|OpenLevel(byName) "None" false))

(event Custom|RestartGameLevel
  (Class|RPGBlueprintLibrary|PlayLoadingScreen true 3.0)
  (CallFunction|LoadGameLevel))

(event Custom|InitItems
  ;[1 1 1] Load All Items
  (bind _keys (Utilities|Map|Keys (Variables|Default|GetItemsPerType)))
  (for _array_element _keys
    (bind _outprimaryassetidlist (Class|KismetSystemLibrary|GetPrimaryAssetIdList _array_element))
    (bind _loaded (|AsyncLoadPrimaryAssetList _outprimaryassetidlist)
      (:Completed
        (for _array_element_2 _loaded
          (bind _asrpgitem (Utilities|Casting|CastToRPGItem _array_element_2))
          (Utilities|Array|Add (Variables|Default|GetStoreItems) _asrpgitem))))))

(event EventInit
  ;[1 1 1] Load All Items
)