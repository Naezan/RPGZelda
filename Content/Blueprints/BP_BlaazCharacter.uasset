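; Blaaz boss character: starts hidden in Peace state, manages split clones, and drives its AI state through a Blackboard enum.
; Splits spawn along three 120-degree directions; regrouped clones reset, re-split, or, when all three arrive in index order, reveal the boss, which then switches to Teleport.
; GAS handles punches, overlap-hit damage events and timed post-hit immunity.
; Death plays global slow motion, then a sequence, and destroys the actor.
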(event OnComponentBeginOverlap(Sphere)
  (params (OverlappedComponent :type Primitive%20Component%20Object%20Reference) (OtherActor :type Actor%20Object%20Reference) (OtherComp :type Primitive%20Component%20Object%20Reference) (OtherBodyIndex :type Integer) (bFromSweep :type Boolean) (SweepResult :type Hit%20Result%20Structure%20%28by%20ref%29))
  ;[1 1 1] 공격체크
  (if (!= (Utilities|GetClass OtherActor) (Utilities|GetClass (Game|GetInstigator)))
    (Utilities|FlowControl|DoOnce false
      (:Completed
        (Ability|SendGameplayEventtoActor self "(TagName=\"Ability.Melee.Damage\")" (Utilities|Struct|MakeGameplayEventData "(TagName=\"\")" (Game|GetInstigator) OtherActor))))))

(event OnComponentEndOverlap(Sphere)
  (params (OverlappedComponent :type Primitive%20Component%20Object%20Reference) (OtherActor :type Actor%20Object%20Reference) (OtherComp :type Primitive%20Component%20Object%20Reference) (OtherBodyIndex :type Integer))
  ;[1 1 1] 공격체크
  (Utilities|FlowControl|Delay 0.2)
  (Utilities|FlowControl|DoOnce false) ; enters at Reset
)

(event Custom|FirstSplit
  ;[1 1 1] 분신 스폰
  (CallFunction|SplitDirection)
  (for _index (range 0 (Variables|Default|GetMaxSpawnCount))
    (bind _output_get (Variables|Default|SetSpawnCount _index))
    (bind _asbp_blaaz_split_character (Utilities|Casting|CastToBP_BlaazSplitCharacterClass (Variables|Default|GetBlaazSplitSpawn)))
    (Game|SpawnActorfromClass _asbp_blaaz_split_character (Math|Transform|MakeTransform (Transformation|GetActorLocation) "0, 0, 0" "1,1,1") "Undefined" 0 _output_get (Utilities|Array|Get(acopy) (Variables|Default|GetFowardSpawnPoint) _output_get) self 0))
  (Collision|SetCollisionResponsetoChannel (Variables|Default|GetCapsuleComponent) "ECC_Pawn" "ECR_Ignore") ; 삭제하지않고 분신들을 관리하는 작업을 계속 진행
  (Collision|SetCollisionResponsetoChannel (Variables|Default|GetCapsuleComponent) "ECC_WorldDynamic" "ECR_Ignore") ; 삭제하지않고 분신들을 관리하는 작업을 계속 진행
  (Development|PrintString "나이아가라 생성"))

(event Custom|SetRandomRotation
  (bind _output_get (Variables|Default|SetDefaultRotation (Math|Rotator|MakeRotator 0.0 0.0 (.Yaw (Math|Rotator|BreakRotator (Math|Random|RandomRotator false))))))
  (Transformation|SetWorldRotation (Variables|Default|Get1) _output_get false false)
  (Transformation|SetWorldRotation (Variables|Default|Get2) (Math|Rotator|CombineRotators (Variables|Default|GetDefaultRotation) (Math|Rotator|MakeRotator 0.0 0.0 1.2e+02)) false false)
  (Transformation|SetWorldRotation (Variables|Default|Get3) (Math|Rotator|CombineRotators (Variables|Default|GetDefaultRotation) (Math|Rotator|MakeRotator 0.0 0.0 2.4e+02)) false false))

(event Custom|Split%20Direction
  ;[1 1 1] 분신 갯수 셋
  (Variables|Default|SetFowardSpawnPoint (Utilities|Array|MakeArray (Math|Vector|GetForwardVector (Variables|Default|Get1)) (Math|Vector|GetForwardVector (Variables|Default|Get2)) (Math|Vector|GetForwardVector (Variables|Default|Get3)))))

(event EventBeginPlay
  (bind _asabp_blaaz (Utilities|Casting|CastToABP_Blaaz (Components|SkeletalMesh|GetAnimInstance (Variables|Character|GetMesh))))
  (Variables|Default|SetAs%20ABP%20Blaaz _asabp_blaaz)
  (Collision|SetCollisionEnabled (Variables|Default|GetSphere) "NoCollision")
  (if (Utilities|Enum|NotEqual(Enum) (Variables|Default|GetBlaazState) "Dead")
    (bind _returnvalue (Class|BlaazCharacter|SetBossState "Peace"))
    (AI|Components|Blackboard|SetValueasEnum (AI|GetBlackboard (AI|GetAIController self)) (Variables|Default|GetKey%20Name) _returnvalue)
    (Rendering|SetActorHiddenInGame true)))

(event EventBoomerangHitCheck
  (bind _splits (Variables|Default|GetSplits))
  (bind _splits_2 (Variables|Default|GetSplits))
  (bind _splits_3 (Variables|Default|GetSplits))
  (bind _splits_4 (Variables|Default|GetSplits))
  ;[1 1 1] 분신 패턴
  (switch int (Utilities|Array|Length (Variables|Default|GetSplits))
    (:1
      (Class|BPIBoss|ResetMovement(Message) (Utilities|Array|Get(acopy) _splits_4))
      (Utilities|Array|Clear _splits_4)
      (Development|PrintString "1마리면 그냥 움직이고 모든거 리셋"))
    (:2
      (for (_array_element _array_index) _splits
        (Variables|/Game/Blueprints/BP_BlaazSplitCharacter.BP_BlaazSplitCharacter_C|SetForward _array_element (* (Math|Vector|GetForwardVector (Variables|Default|GetDefaultRotation)) (Math|Integer|SelectInt 1 -1 (== _array_index 0))))
        (Default|SelfSplit _array_element)
        (Development|PrintString "2마리 뭉침"))
      (Utilities|Array|Clear _splits))
    (:3
      (Utilities|FlowControl|Delay 2.0)
      (for (_array_element_2 _array_index_2) _splits_2
        (if (== (Variables|/Game/Blueprints/BP_BlaazSplitCharacter.BP_BlaazSplitCharacter_C|GetIndex _array_element_2) _array_index_2)
          (Math|Integer|IncrementInt (Variables|Default|GetCorrectCount))))
      (if (== (Utilities|Array|Length _splits_2) (Variables|Default|GetCorrectCount)) ; 3마리 뭉친경우
        (Transformation|SetActorLocation (Variables|Default|GetBossSpawnPoint) false false)
        (for _array_element_3 (Variables|Default|GetSplits)
          (Actor|DestroyActor _array_element_3))
        (Utilities|Array|Clear (Variables|Default|GetSplits))
        (Development|PrintString "보스 소환")
        (Variables|Default|SetCorrectCount 0)
        (Rendering|SetActorHiddenInGame false)
        (Collision|SetCollisionProfileName (Variables|Default|GetCapsuleComponent) "Pawn" true :!class /Script/Engine.PrimitiveComponent)
        (Animation|Montage|PlayMontage (Variables|Character|GetMesh) "/Game/Monsters/Blaaz/Animations/Montage/Appear_Montage.Appear_Montage"
          (:then
            (Development|PrintString "등장 애니메이션도중 한1초?동안은 무적"))
          (:OnBlendOut
            (Utilities|FlowControl|Delay 3.0)
            (bind _returnvalue (Class|BlaazCharacter|SetBossState "Teleport"))
            (AI|Components|Blackboard|SetValueasEnum (AI|GetBlackboard (AI|GetAIController self)) (Variables|Default|GetKey%20Name) _returnvalue)))
        (else
          (CallFunction|SetRandomRotation)
          (for _array_element_4 _splits_3
            (Default|SelfSplit _array_element_4) ; 타임라인 왜 재생안됨?
          )
          (Utilities|Array|Clear _splits_3)
          (Development|PrintString "다시 퍼짐")
          (Variables|Default|SetCorrectCount 0))))))

(event EventOnDamaged
  (params (DamageAmount :type Float%20%28single-precision%29) (HitInfo :type Hit%20Result%20Structure%20%28by%20ref%29) (DamageTags :type Gameplay%20Tag%20Container%20Structure%20%28by%20ref%29) (InstigatorCharacter :type Character%20Base%20Object%20Reference) (DamageCauser :type Actor%20Object%20Reference))
  (bind _returnvalue (Class|CharacterBase|GetHealth))
  (bind _deadsequence (Variables|Default|GetDeadSequence))
  (if (not (Variables|Default|GetIsDead))
    (Variables|Default|SetDamagedAmount (+ (Variables|Default|GetDamagedAmount) DamageAmount))
    (Utilities|FlowControl|Sequence
      (:then_0
        (Audio|PlaySound2D "/Game/Assets/Sounds/AttackSound.AttackSound" 1.0 1.0 0.0 0 0)
        (if (> _returnvalue 0.1)
          (Development|PrintString (Utilities|String|ToString(Float) _returnvalue))
          (else
            (bind _returnvalue_2 (Class|BlaazCharacter|SetBossState "Dead"))
            (AI|Components|Blackboard|SetValueasEnum (AI|GetBlackboard (AI|GetAIController self)) (Variables|Default|GetKey%20Name) _returnvalue_2)
            (Variables|Default|SetIsDead true)
            (bind _새_트랙_0 (Timeline|SlowMotion PlayFromStart) ; 맞을떄 그상태에선 슬로우
              (:Update
                (Utilities|Time|SetGlobalTimeDilation _새_트랙_0))
              (:Finished
                (Sequencer|Player|Play (Variables|/Script/LevelSequence.LevelSequenceActor|GetSequencePlayer _deadsequence) :!class /Script/MovieScene.MovieSceneSequencePlayer) ; 보스 죽음 시퀀서 재생
                (Development|PrintString (Utilities|GetDisplayName _deadsequence))
                (Actor|DestroyActor))))))
      (:then_1
        (Development|PrintString "무적 어빌리티 활성화")
        (GameplayEffects|ApplyGameplayEffectToSelf :self (Variables|Default|GetAbilitySystemComponent) :GameplayEffectClass (Variables|Default|GetDamageImmune))
        (bind _새_트랙_0_2 (Timeline|타임라인_0 PlayFromStart)
          (:Update
            (Variables|Default|SetBoneScale _새_트랙_0_2))
          (:Finished
            (Variables|Default|SetBoneScale 0.0)
            (Development|PrintString "무적 어빌리티 비활성화")
            (GameplayEffects|RemoveActiveGameplayEffectbySourceEffect (Variables|Default|GetAbilitySystemComponent) (Variables|Default|GetDamageImmune) 0 -1)))))))

(event EventOnAttacking
  (Abilities|TryActivateAbilitybyClass (Variables|Default|GetAbilitySystemComponent) "/Game/Abilities/Enemies/Blaaz/GA_BlaazPunch.GA_BlaazPunch_C" true))

(event EventEventBeginAttack
  (Collision|SetCollisionEnabled (Variables|Default|GetSphere) "QueryOnly"))

(event EventEventEndAttack
  (Utilities|FlowControl|Delay 0.2)
  (Collision|SetCollisionEnabled (Variables|Default|GetSphere) "NoCollision"))

(fn ConstructionScript)