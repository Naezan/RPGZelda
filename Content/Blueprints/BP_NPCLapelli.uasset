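; BP_NPCLapelli is the Lapelli NPC Blueprint that drives the character's encounter, dialogue and procedural head-turn animation.
; Its events cast the mesh's anim instance to ABP_Lapelli and set variables for head rotation, its blend alpha and talking state.
; InteractiveCollision overlap with BP_LinkCharacter starts the encounter state.
; Ending interaction clears encounter and talking flags and pulses IsDone for 0.2 seconds.
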(event OnComponentBeginOverlap(InteractiveCollision)
  (params (OverlappedComponent :type Primitive%20Component%20Object%20Reference) (OtherActor :type Actor%20Object%20Reference) (OtherComp :type Primitive%20Component%20Object%20Reference) (OtherBodyIndex :type Integer) (bFromSweep :type Boolean) (SweepResult :type Hit%20Result%20Structure%20%28by%20ref%29))
  ;[1 1 1] 캐릭터 대화 시작
  (if (== (Utilities|GetClass OtherActor) "/Game/Blueprints/BP_LinkCharacter.BP_LinkCharacter_C")
    (bind _asabp_lapelli (Utilities|Casting|CastToABP_Lapelli (Components|SkeletalMesh|GetAnimInstance (Variables|Character|GetMesh))))
    (Variables|/Game/Characters/Lapelli/ABP_Lapelli.ABP_Lapelli_C|SetIsEncounter _asabp_lapelli true)))

(event EventBeginPlay)

(event Collision|EventActorBeginOverlap
  (params (OtherActor :type Actor%20Object%20Reference)))

(event EventTick
  (params (DeltaSeconds :type Float%20%28single-precision%29)))

(event EventSetInteractBeginAnimation
  ;[1 1 1] 대화 애니메이션
  (bind _asabp_lapelli (Utilities|Casting|CastToABP_Lapelli (Components|SkeletalMesh|GetAnimInstance (Variables|Character|GetMesh))))
  (Variables|/Game/Characters/Lapelli/ABP_Lapelli.ABP_Lapelli_C|SetIsTalking _asabp_lapelli true))

(event EventSetHeadRotationAlpha
  (params (alpha :type Float%20%28single-precision%29))
  ;[1 1 1] 캐릭터 절차적 머리 회전
  (bind _asabp_lapelli (Utilities|Casting|CastToABP_Lapelli (Components|SkeletalMesh|GetAnimInstance (Variables|Character|GetMesh))))
  (Variables|/Game/Characters/Lapelli/ABP_Lapelli.ABP_Lapelli_C|SetRotationHeadAlpha _asabp_lapelli alpha))

(event EventSetHeadRotation
  (params (rotator :type Rotator :default "0, 0, 0"))
  ;[1 1 1] 캐릭터 절차적 머리 회전
  (bind _asabp_lapelli (Utilities|Casting|CastToABP_Lapelli (Components|SkeletalMesh|GetAnimInstance (Variables|Character|GetMesh))))
  (Variables|/Game/Characters/Lapelli/ABP_Lapelli.ABP_Lapelli_C|SetHeadRotation _asabp_lapelli rotator))

(event EventSetInteractEndAnimation
  ;[1 1 1] 대화 애니메이션
  (bind _asabp_lapelli (Utilities|Casting|CastToABP_Lapelli (Components|SkeletalMesh|GetAnimInstance (Variables|Character|GetMesh))))
  (Variables|/Game/Characters/Lapelli/ABP_Lapelli.ABP_Lapelli_C|SetIsDone _asabp_lapelli true)
  (Variables|/Game/Characters/Lapelli/ABP_Lapelli.ABP_Lapelli_C|SetIsEncounter _asabp_lapelli false)
  (Variables|/Game/Characters/Lapelli/ABP_Lapelli.ABP_Lapelli_C|SetIsTalking _asabp_lapelli false)
  (Utilities|FlowControl|Delay 0.2)
  (Variables|/Game/Characters/Lapelli/ABP_Lapelli.ABP_Lapelli_C|SetIsDone _asabp_lapelli false))

(fn ConstructionScript)