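; Boss chest interactable that gives Link an item in a Zelda-style RPG, revealed by ShowChest with a poof effect.
; Interacting opens the lid through an Alpha on ABP_BigChest, while Tick moves the player to the pickup point.
; Chained montages drive the camera zoom, item-get sound, dialogue and item mesh spawn, with another montage when dialogue ends.
; A valid AcquireItem is added to Link's equipment, spawned as a weapon and saved through the game mode.
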(event Custom|ShowChest
  (Rendering|SetActorHiddenInGame false)
  (Niagara|SpawnSystematLocation "/Game/FX/FX_Poof/NS_Poof.NS_Poof" (Transformation|GetWorldLocation (Variables|Default|GetNiagaraPosition))))

(event EventBeginPlay
  (Utilities|FlowControl|Delay 0.2)
  (CallFunction|OpenChest (Variables|Default|GetAlpha)))

(event EventTick
  (params (DeltaSeconds :type Float%20%28single-precision%29))
  (if (and (Variables|Default|GetbIsInteract) (not (Variables|Default|GetMoveComplete)))
    (Class|QuestChestActor|MovetoPickUpPoint (Variables|Default|GetInstigator%20Pawn) DeltaSeconds)
    (if (Variables|Default|GetMoveComplete)
      (Actor|Tick|SetActorTickEnabled false))))

(event EventInteract
  (params (InstigatorPawn :type Pawn%20Object%20Reference))
  (bind _acquireitem (Variables|Default|GetAcquireItem))
  (if (not (Variables|Default|GetbIsInteract))
    (Variables|Default|SetbIsInteract true)
    (|CallParentFunction InstigatorPawn)
    (bind _output_get (Variables|Default|SetAlpha 1.0))
    (CallFunction|OpenChest _output_get)
    (Audio|PlaySound2D "/Game/Assets/Sounds/OpenChest.OpenChest" 1.0 1.0 0.0 0 0)
    (bind _output_get_2 (Variables|Default|SetInstigator%20Pawn InstigatorPawn))
    (bind _asbp_link_character (Utilities|Casting|CastToBP_LinkCharacter _output_get_2))
    (Animation|Montage|PlayMontage (Variables|/Script/Engine.Character|GetMesh _asbp_link_character) "/Game/Characters/Link/Animations/Montages/boxopen_Montage.boxopen_Montage"
      (:OnCompleted
        (Class|QuestChestActor|ZoominCamera)
        (Animation|Montage|PlayMontage (Variables|/Script/Engine.Character|GetMesh _asbp_link_character) "/Game/Characters/Link/Animations/Montages/itemget_Montage.itemget_Montage"
          (:then
            (Audio|PlaySound2D "/Game/Assets/Sounds/Get_Item.Get_Item" 1.0 1.0 0.0 0 0)
            (bind _returnvalue (Animation|GetPlayLength (Variables|Default|GetItemGetMontage)))
            (Utilities|FlowControl|Delay _returnvalue)
            (Class|QuestChestActor|InteractDialogue)
            ;[1 1 1] 장비가 있다면 장착
            (Class|QuestChestActor|SpawnStaticMeshActor (Transformation|GetWorldLocation (Variables|Default|GetItemSpawnPoint)))
            (Utilities|IsValid (Variables|Default|GetAcquireItem)
              (:Is%20Valid
                (bind _returnvalue_2 (Utilities|Array|Add (Variables|/Script/RPGZelda.LinkCharacter|GetEquippedRPGItems _asbp_link_character) _acquireitem))
                (bind _asrpgweapon_item (Utilities|Casting|CastToRPGWeaponItem _acquireitem))
                (bind _asbp_weapon (Utilities|Casting|CastToBP_WeaponClass (Variables|/Script/RPGZelda.RPGWeaponItem|GetWeaponActor _asrpgweapon_item)))
                (bind _returnvalue_3 (Game|SpawnActorfromClass _asbp_weapon (Math|Transform|MakeTransform "0, 0,-1000.000000") "Undefined" 0 _asrpgweapon_item (Utilities|Struct|MakeRPGItemInfo "Weapon" _returnvalue_2) 0))
                (Utilities|Array|Add (Variables|/Game/Blueprints/BP_LinkCharacter.BP_LinkCharacter_C|GetEquippedWeapons _asbp_link_character) _returnvalue_3)
                (bind _asbp_rpgzelda_game_mode (Utilities|Casting|CastToBP_RPGZeldaGameMode (Game|GetGameMode)))
                (Default|SaveGame _asbp_rpgzelda_game_mode)))))))))

(event EventDialogueAnimEnd
  (bind _asbp_link_character (Utilities|Casting|CastToBP_LinkCharacter (Variables|Default|GetInstigator%20Pawn)))
  (Animation|Montage|PlayMontage (Variables|/Script/Engine.Character|GetMesh _asbp_link_character) "/Game/Characters/Link/Animations/Montages/powdown_Montage.powdown_Montage"))

(fn ConstructionScript)

(fn OpenChest
  (params (Alpha :type Float%20%28single-precision%29))
  (bind _asabp_big_chest (Utilities|Casting|CastToABP_BigChest (Components|SkeletalMesh|GetAnimInstance (Variables|Default|GetMeshComp))))
  (Variables|/Game/Objects/Chest/Big/ABP_BigChest.ABP_BigChest_C|SetAlpha _asabp_big_chest Alpha))