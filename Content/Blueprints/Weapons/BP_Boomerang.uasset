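; Boomerang weapon that records a mouse-drawn path during an attack and throws a boomerang when it ends.
; KeepAttack adds cursor points to the player controller, projecting trace results onto the boomerang's height plane and messaging hit actors to stop moving.
; EndAttack plays the throw montage, hides the mesh and spawns BP_Boom.
; The character's movement lock from BeginAttack lifts and the mesh reappears when BP_Boom is destroyed.
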(event Custom|ShowMesh
  (params (DestroyedActor :type Actor%20Object%20Reference))
  (Variables|/Script/RPGZelda.LinkCharacter|SetbIsStopMoving (Variables|Default|GetMyCharacter) false)
  (Rendering|SetVisibility (Variables|Character|GetMesh) true false))

(event EventBeginPlay
  (|CallParentFunction)
  (bind _asbp_rpgplayer_controller (Utilities|Casting|CastToBP_RPGPlayerController (Game|GetPlayerController 0)))
  (Variables|Default|SetAs%20BP%20RPGPlayer%20Controller _asbp_rpgplayer_controller))

(event Collision|EventActorBeginOverlap
  (params (OtherActor :type Actor%20Object%20Reference))
  (|CallParentFunction OtherActor) ; 지금 이 노드는 비활성 상태입니다. \n핀을 끌어서 다른 노드를 연결하면 활성화됩니다.
)

(event EventBeginAttack
  (bind _mycharacter (Variables|Default|GetMyCharacter))
  (Variables|/Script/RPGZelda.CharacterBase|SetIsAttacking _mycharacter true)
  (Variables|/Script/RPGZelda.LinkCharacter|SetbIsStopMoving _mycharacter true))

(event EventKeepAttack
  (bind _as_bp_rpgplayer_controller (Variables|Default|GetAs%20BP%20RPGPlayer%20Controller))
  (bind _as_bp_rpgplayer_controller_2 (Variables|Default|GetAs%20BP%20RPGPlayer%20Controller))
  (bind _as_bp_rpgplayer_controller_3 (Variables|Default|GetAs%20BP%20RPGPlayer%20Controller))
  (bind _boomposition (Variables|Default|GetBoomPosition))
  (bind (_worldlocation _worlddirection) (Game|Player|ConvertMouseLocationToWorldSpace _as_bp_rpgplayer_controller_3))
  (bind _returnvalue (Transformation|GetWorldLocation _boomposition))
  (bind (_locationx _locationy) (Class|WidgetLayoutLibrary|GetMousePositionScaledbyDPI _as_bp_rpgplayer_controller))
  (bind _drawing (Variables|/Game/Blueprints/BP_RPGPlayerController.BP_RPGPlayerController_C|GetDrawing _as_bp_rpgplayer_controller_2))
  (bind _z (Math|Vector|BreakVector _returnvalue))
  (bind _returnvalue_2 (Math|Vector2D|MakeVector2D _locationx _locationy))
  (bind _points (Variables|/Game/UI/WBP_Drawing.WBP_Drawing_C|GetPoints _drawing))
  ;[1 1 1] 라인 포지션 설정과 부메랑위치 조정
  (Utilities|IsValid (Variables|Default|GetMyCharacter)
    (:Is%20Valid
      (if (> (Utilities|Array|Length (Variables|/Game/UI/WBP_Drawing.WBP_Drawing_C|GetPoints (Variables|/Game/Blueprints/BP_RPGPlayerController.BP_RPGPlayerController_C|GetDrawing (Variables|Default|GetAs%20BP%20RPGPlayer%20Controller)))) 0)
        (if (not (Math|Vector|Equal(Vector) (Utilities|Array|Get(acopy) _points (Utilities|Array|LastIndex _points)) _returnvalue_2 0.1))
          (Utilities|Array|Add (Variables|/Game/UI/WBP_Drawing.WBP_Drawing_C|GetPoints (Variables|/Game/Blueprints/BP_RPGPlayerController.BP_RPGPlayerController_C|GetDrawing (Variables|Default|GetAs%20BP%20RPGPlayer%20Controller))) _returnvalue_2 :!label _label)
          ;;[1 1 1] 디버그용
          (bind _outhit (Collision|LineTraceByChannel _worldlocation (+ _worldlocation (* _worlddirection 1e+03)) "TraceTypeQuery1" false 0 "None"))
          (Utilities|Array|Add (Variables|/Game/Blueprints/BP_RPGPlayerController.BP_RPGPlayerController_C|GetLocation (Variables|Default|GetAs%20BP%20RPGPlayer%20Controller)) (Math|Vector|MakeVector (+ (/ (- (.X (Math|Vector|BreakVector (.Location (Collision|BreakHitResult _outhit)))) (.X (Math|Vector|BreakVector (.TraceStart (Collision|BreakHitResult _outhit))))) (/ (- (.Z (Math|Vector|BreakVector (.Location (Collision|BreakHitResult _outhit)))) (.Z (Math|Vector|BreakVector (.TraceStart (Collision|BreakHitResult _outhit))))) (- _z (.Z (Math|Vector|BreakVector (.TraceStart (Collision|BreakHitResult _outhit))))))) (.X (Math|Vector|BreakVector (.TraceStart (Collision|BreakHitResult _outhit))))) (+ (/ (- (.Y (Math|Vector|BreakVector (.Location (Collision|BreakHitResult _outhit)))) (.Y (Math|Vector|BreakVector (.TraceStart (Collision|BreakHitResult _outhit))))) (/ (- (.Z (Math|Vector|BreakVector (.Location (Collision|BreakHitResult _outhit)))) (.Z (Math|Vector|BreakVector (.TraceStart (Collision|BreakHitResult _outhit))))) (- _z (.Z (Math|Vector|BreakVector (.TraceStart (Collision|BreakHitResult _outhit))))))) (.Y (Math|Vector|BreakVector (.TraceStart (Collision|BreakHitResult _outhit))))) _z))
          (Class|BPIWeapon|StopMoveCharacter(Message) (.HitActor (Collision|BreakHitResult _outhit))))
        (else
          (goto _label))))))

(event EventEndAttack
  (bind _mycharacter (Variables|Default|GetMyCharacter))
  (Animation|Montage|PlayMontage (Variables|/Script/Engine.Character|GetMesh (Variables|Default|GetMyCharacter)) "/Game/Characters/Link/Animations/Montages/boomthrow_Montage.boomthrow_Montage"
    (:then
      (Rendering|SetVisibility (Variables|Character|GetMesh) false false)
      (Development|PrintString "파티클들 삭제")
      (bind _returnvalue (Game|SpawnActorfromClass "/Game/Blueprints/Weapons/BP_Boom.BP_Boom_C" (Math|Transform|MakeTransform (Transformation|GetWorldLocation (Variables|Default|GetBoomPosition)) (Transformation|GetActorRotation _mycharacter) "1,1,1") "Undefined" 0 _mycharacter))
      (Game|BindEventtoOnDestroyed _returnvalue (delegate Custom|ShowMesh)))))

(fn ConstructionScript
  (|CallParentFunction))