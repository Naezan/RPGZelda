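; BP_Boom is a boomerang weapon that flies along the path drawn on the player controller, returns to the player, then destroys itself and calls Enable on the controller.
; Timelines ease it to the start and back, while Tick steps it through the stored points.
; Blaaz split actors it touches are dragged along and reported to their parent boss at path end.
; Other valid hits run parent overlap logic, clear the drawing and trigger the return.
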(event Custom|InputEnable
  (params (DestroyedActor :type Actor%20Object%20Reference))
  (Class|RPGPlayerController|Enable (Variables|Default|GetAs%20BP%20RPGPlayer%20Controller)))

(event EventBeginPlay
  (bind _asbp_rpgplayer_controller (Utilities|Casting|CastToBP_RPGPlayerController (Game|GetPlayerController 0)))
  (Variables|Default|SetAs%20BP%20RPGPlayer%20Controller _asbp_rpgplayer_controller)
  (Game|BindEventtoOnDestroyed (delegate Custom|InputEnable)))

(event Collision|EventActorBeginOverlap
  (params (OtherActor :type Actor%20Object%20Reference))
  (bind _returnvalue (Utilities|GetClass OtherActor))
  (bind _splitactors (Variables|Default|GetSplitActors))
  (if (and (!= _returnvalue "/Game/Blueprints/BP_LinkCharacter.BP_LinkCharacter_C") (!= _returnvalue (Utilities|GetClass (Variables|Default|GetInstigator))))
    (if (and (== _returnvalue "/Game/Blueprints/BP_BlaazSplitCharacter.BP_BlaazSplitCharacter_C") (!= _returnvalue "/Game/Blueprints/BP_BlaazCharacter.BP_BlaazCharacter_C")) ; 특수보스인지 일반몹인지 체크
      (if (== (Utilities|Array|FindItem _splitactors OtherActor) -1)
        (Utilities|Array|Add _splitactors OtherActor))
      (else
        (CallFunction|ClearDraw)
        (|CallParentFunction OtherActor)
        ;[1 1 1] 플레이어 지점 이동
        (Timeline|MoveToPlayer Play
          (:Update
            (Transformation|SetActorLocation (Math|Interpolation|VInterpTo (Transformation|GetActorLocation) (Transformation|GetActorLocation (Variables|/Game/Blueprints/BP_RPGPlayerController.BP_RPGPlayerController_C|GetPlayer%20Character (.AsBP%20RPGPlayer%20Controller (Utilities|Casting|CastToBP_RPGPlayerController (Game|GetPlayerController 0))))) (Utilities|Time|GetWorldDeltaSeconds) 5.0) false false))
          (:Finished
            (Actor|DestroyActor)))))))

(event EventTick
  (params (DeltaSeconds :type Float%20%28single-precision%29))
  (bind _locationidx (Variables|Default|GetLocationIdx))
  (bind _as_bp_rpgplayer_controller (Variables|Default|GetAs%20BP%20RPGPlayer%20Controller))
  (bind _location (Variables|/Game/Blueprints/BP_RPGPlayerController.BP_RPGPlayerController_C|GetLocation _as_bp_rpgplayer_controller))
  (bind _output (Utilities|Array|Get(acopy) _location _locationidx))
  (Utilities|IsValid _as_bp_rpgplayer_controller
    (:Is%20Valid
      ;[1 1 1] 스타트지점 이동
      (if (Utilities|Array|IsValidIndex _location)
        (Timeline|MoveToStart Play
          (:Update
            (Transformation|SetActorLocation (Math|Interpolation|VInterpTo (Transformation|GetActorLocation) (Utilities|Array|Get(acopy) _location) DeltaSeconds 15.0) false false))
          (:Finished
            ;[1 1 1] 선따라 이동
            (if (> (Variables|Default|GetLocationIdx) (Utilities|Array|LastIndex _location))
              (CallFunction|SendSplittoBlazz)
              (CallFunction|ClearDraw)
              (Utilities|Array|Clear (Variables|Default|GetSplitActors)) ; 한번 실행됨
              ;[1 1 1] 플레이어 지점 이동
              (Timeline|MoveToPlayer Play
                (:Update
                  (Transformation|SetActorLocation (Math|Interpolation|VInterpTo (Transformation|GetActorLocation) (Transformation|GetActorLocation (Variables|/Game/Blueprints/BP_RPGPlayerController.BP_RPGPlayerController_C|GetPlayer%20Character (.AsBP%20RPGPlayer%20Controller (Utilities|Casting|CastToBP_RPGPlayerController (Game|GetPlayerController 0))))) (Utilities|Time|GetWorldDeltaSeconds) 5.0) false false))
                (:Finished
                  (Actor|DestroyActor)))
              (else
                (Transformation|SetActorLocation _output false false)
                (for _array_element (Variables|Default|GetSplitActors) ; 보스오브젝트 부메랑따라가기
                  (Transformation|SetActorLocation _array_element _output false false))
                (Math|Integer|IncrementInt (Variables|Default|GetLocationIdx))))))))))

(fn ConstructionScript
  (|CallParentFunction))

(fn ClearDraw
  (bind _as_bp_rpgplayer_controller (Variables|Default|GetAs%20BP%20RPGPlayer%20Controller))
  (Utilities|Array|Clear (Variables|/Game/Blueprints/BP_RPGPlayerController.BP_RPGPlayerController_C|GetLocation _as_bp_rpgplayer_controller))
  (Utilities|Array|Clear (Variables|/Game/UI/WBP_Drawing.WBP_Drawing_C|GetPoints (Variables|/Game/Blueprints/BP_RPGPlayerController.BP_RPGPlayerController_C|GetDrawing _as_bp_rpgplayer_controller))))

(fn SendSplittoBlazz
  (bind _as_bp_rpgplayer_controller (Variables|Default|GetAs%20BP%20RPGPlayer%20Controller))
  (bind _splitactors (Variables|Default|GetSplitActors))
  (bind _location (Variables|/Game/Blueprints/BP_RPGPlayerController.BP_RPGPlayerController_C|GetLocation _as_bp_rpgplayer_controller))
  (if (Utilities|Array|IsValidIndex _splitactors)
    (for _array_element _splitactors
      (bind _asbp_blaaz_split_character (Utilities|Casting|CastToBP_BlaazSplitCharacter _array_element))
      (Utilities|Array|Add (Variables|/Game/Blueprints/BP_BlaazCharacter.BP_BlaazCharacter_C|GetSplits (Variables|/Game/Blueprints/BP_BlaazSplitCharacter.BP_BlaazSplitCharacter_C|GetParentBoss _asbp_blaaz_split_character)) _asbp_blaaz_split_character)
      (Variables|/Game/Blueprints/BP_BlaazCharacter.BP_BlaazCharacter_C|SetBossSpawnPoint (Variables|/Game/Blueprints/BP_BlaazSplitCharacter.BP_BlaazSplitCharacter_C|GetParentBoss _asbp_blaaz_split_character) (Utilities|Array|Get(acopy) _location (Utilities|Array|LastIndex _location))))
    (Class|BPIWeapon|BoomerangHitCheck(Message) (Variables|/Game/Blueprints/BP_BlaazSplitCharacter.BP_BlaazSplitCharacter_C|GetParentBoss _asbp_blaaz_split_character))))