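; Base projectile for ranged abilities that reports a hit when it overlaps another actor.
; Overlaps with BP_LinkCharacter or actors of the Instigator's class are ignored.
; The first valid hit sends an Ability.Ranged.Damage gameplay event to player 0's character, naming it as instigator and the hit actor as target.
; A DoOnce limits this to one hit, which also spawns a P_Bomb effect at the projectile's location.
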(event Collision|EventActorBeginOverlap
  (params (OtherActor :type Actor%20Object%20Reference))
  (bind _returnvalue (Utilities|GetClass OtherActor))
  (bind _returnvalue_2 (Game|GetPlayerController 0))
  (bind (_asbp_rpgplayer_controller _bsuccess) (Utilities|Casting|CastToBP_RPGPlayerController _returnvalue_2))
  (bind _player_character (Variables|/Game/Blueprints/BP_RPGPlayerController.BP_RPGPlayerController_C|GetPlayer%20Character _asbp_rpgplayer_controller))
  (if (and (!= _returnvalue "/Game/Blueprints/BP_LinkCharacter.BP_LinkCharacter_C") (!= _returnvalue (Utilities|GetClass (Variables|Actor|GetInstigator))))
    (if _bsuccess
      (Utilities|IsValid _player_character
        (:Is%20Valid
          (Utilities|FlowControl|DoOnce false
            (:Completed
              (Ability|SendGameplayEventtoActor _player_character "(TagName=\"Ability.Ranged.Damage\")" (Utilities|Struct|MakeGameplayEventData "(TagName=\"\")" _player_character OtherActor))
              (Effects|SpawnEmitteratLocation "/Game/FX/FX_Mobile/P_Bomb.P_Bomb" (Transformation|GetActorLocation)))))))))

(fn ConstructionScript)