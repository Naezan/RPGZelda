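; Bow weapon that lets its owning character draw, aim and fire arrows through begin, keep and end attack events.
; BeginAttack flags the character as attacking and shows the nocked arrow mesh, which construction hides, while KeepAttack rotates the character.
; EndAttack starts the shoot montage, then immediately hides that mesh and spawns BP_Arrow at ArrowPosition, facing the character's rotation with the character as instigator.
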(event EventBeginPlay
  (|CallParentFunction) ; 지금 이 노드는 비활성 상태입니다. \n핀을 끌어서 다른 노드를 연결하면 활성화됩니다.
)

(event Collision|EventActorBeginOverlap
  (params (OtherActor :type Actor%20Object%20Reference))
  (|CallParentFunction OtherActor) ; 지금 이 노드는 비활성 상태입니다. \n핀을 끌어서 다른 노드를 연결하면 활성화됩니다.
)

(event EventEndAttack
  (bind _mycharacter (Variables|Default|GetMyCharacter))
  (Animation|Montage|PlayMontage (Variables|/Script/Engine.Character|GetMesh (Variables|Default|GetMyCharacter)) "/Game/Characters/Link/Animations/Montages/arrowshoot_Montage.arrowshoot_Montage"
    (:then
      (Rendering|SetVisibility (Variables|Default|GetArrowMesh) false false)
      (Game|SpawnActorfromClass "/Game/Blueprints/Weapons/BP_Arrow.BP_Arrow_C" (Math|Transform|MakeTransform (Transformation|GetWorldLocation (Variables|Default|GetArrowPosition)) (Transformation|GetActorRotation _mycharacter) "1,1,1") "Undefined" 0 _mycharacter))))

(event EventBeginAttack
  (Variables|/Script/RPGZelda.CharacterBase|SetIsAttacking (Variables|Default|GetMyCharacter) true)
  (Rendering|SetVisibility (Variables|Default|GetArrowMesh) true false))

(event EventKeepAttack
  (bind _mycharacter (Variables|Default|GetMyCharacter))
  (Utilities|IsValid _mycharacter
    (:Is%20Valid
      (Class|LinkCharacter|RotateCharacter _mycharacter))))

(fn ConstructionScript
  (|CallParentFunction)
  (Rendering|SetVisibility (Variables|Default|GetArrowMesh) false false))