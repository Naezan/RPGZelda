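; BP_Bomb is a bomb weapon that its owning character throws by spawning a separate projectile actor.
; BeginAttack flags the character as attacking, and EndAttack starts the grab-throw montage and immediately hides the bomb mesh without waiting for completion.
; It then spawns BP_ThrowBomb at BombPosition with the character's rotation and as its instigator.
; The thrown bomb's OnDestroyed event makes the held mesh visible again.
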(event Custom|ShowMesh
  (params (DestroyedActor :type Actor%20Object%20Reference))
  (Rendering|SetVisibility (Variables|Character|GetMesh) true false))

(event EventBeginPlay
  (|CallParentFunction) ; 지금 이 노드는 비활성 상태입니다. \n핀을 끌어서 다른 노드를 연결하면 활성화됩니다.
)

(event Collision|EventActorBeginOverlap
  (params (OtherActor :type Actor%20Object%20Reference))
  (|CallParentFunction OtherActor) ; 지금 이 노드는 비활성 상태입니다. \n핀을 끌어서 다른 노드를 연결하면 활성화됩니다.
)

(event EventTick
  (params (DeltaSeconds :type Float%20%28single-precision%29)))

(event EventBeginAttack
  (Variables|/Script/RPGZelda.CharacterBase|SetIsAttacking (Variables|Default|GetMyCharacter) true))

(event EventEndAttack
  (bind _mycharacter (Variables|Default|GetMyCharacter))
  (Animation|Montage|PlayMontage (Variables|/Script/Engine.Character|GetMesh (Variables|Default|GetMyCharacter)) "/Game/Characters/Link/Animations/Montages/grabthrow_Montage.grabthrow_Montage"
    (:then
      (Rendering|SetVisibility (Variables|Character|GetMesh) false false)
      (Development|PrintString "파티클들 삭제")
      (bind _returnvalue (Game|SpawnActorfromClass "/Game/Abilities/Player/Bomb/BP_ThrowBomb.BP_ThrowBomb_C" (Math|Transform|MakeTransform (Transformation|GetWorldLocation (Variables|Default|GetBombPosition)) (Transformation|GetActorRotation _mycharacter) "1,1,1") "Undefined" 0 _mycharacter))
      (Game|BindEventtoOnDestroyed _returnvalue (delegate Custom|ShowMesh)))))

(fn ConstructionScript
  (|CallParentFunction))