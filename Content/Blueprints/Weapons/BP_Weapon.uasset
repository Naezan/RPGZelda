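; BP_Weapon is a melee weapon actor that reports hits to its BP_LinkCharacter through the Gameplay Ability System.
; Attack begin and end events toggle capsule query collision, with a short delay before disabling.
; Overlaps, excluding BP_LinkCharacter and the instigator's class, send an Ability.Melee.Damage gameplay event to that character with the hit actor as target.
; A DoOnce limits repeat hits until shortly after an overlap ends.
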(event Custom|EventEndWeaponAttack
  (Utilities|FlowControl|Delay 0.2)
  (Collision|SetCollisionEnabled (Variables|Default|GetCapsuleComp) "NoCollision"))

(event Custom|EventBeginWeaponAttack
  (Collision|SetCollisionEnabled (Variables|Default|GetCapsuleComp) "QueryOnly"))

(event EventBeginPlay)

(event Collision|EventActorBeginOverlap
  (params (OtherActor :type Actor%20Object%20Reference))
  (bind _returnvalue (Utilities|GetClass OtherActor))
  (bind _mycharacter (Variables|Default|GetMyCharacter))
  (bind _asbp_link_character (Utilities|Casting|CastToBP_LinkCharacter _mycharacter))
  ;[1 1 1] 충돌하게 되면 나의 부모오브젝트에 데미지이벤트를 발생시켜라
  (if (and (!= _returnvalue "/Game/Blueprints/BP_LinkCharacter.BP_LinkCharacter_C") (!= _returnvalue (Utilities|GetClass (Game|GetInstigator))))
    (Utilities|FlowControl|DoOnce false
      (:Completed
        (Ability|SendGameplayEventtoActor _asbp_link_character "(TagName=\"Ability.Melee.Damage\")" (Utilities|Struct|MakeGameplayEventData "(TagName=\"\")" _asbp_link_character OtherActor))))))

(event Collision|EventActorEndOverlap
  (params (OtherActor :type Actor%20Object%20Reference))
  (bind _mycharacter (Variables|Default|GetMyCharacter))
  (bind _asbp_link_character (Utilities|Casting|CastToBP_LinkCharacter _mycharacter))
  ;[1 1 1] 충돌하게 되면 나의 부모오브젝트에 데미지이벤트를 발생시켜라
  (Utilities|FlowControl|Delay 0.2)
  (Utilities|FlowControl|DoOnce false) ; enters at Reset
)

(fn ConstructionScript)