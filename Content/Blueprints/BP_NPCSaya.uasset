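; BP_NPCSaya is the Saya NPC Blueprint, which drives the character's procedural head turning and dialogue animation.
; Its events cast the mesh's anim instance to ABP_Saya and write head rotation, head rotation alpha and talking state into it.
; Ending an interaction clears IsTalking and pulses IsDone, resetting it after a short delay.
; BeginPlay, Tick, overlap and the construction script are empty.
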(event EventBeginPlay)

(event Collision|EventActorBeginOverlap
  (params (OtherActor :type Actor%20Object%20Reference)))

(event EventTick
  (params (DeltaSeconds :type Float%20%28single-precision%29)))

(event EventSetInteractBeginAnimation
  ;[1 1 1] 대화 애니메이션
  (bind _asabp_saya (Utilities|Casting|CastToABP_Saya (Components|SkeletalMesh|GetAnimInstance (Variables|Character|GetMesh))))
  (Variables|/Game/Characters/Saya/ABP_Saya.ABP_Saya_C|SetIsTalking _asabp_saya true))

(event EventSetHeadRotationAlpha
  (params (alpha :type Float%20%28single-precision%29))
  ;[1 1 1] 캐릭터 절차적 머리 회전
  (bind _asabp_saya (Utilities|Casting|CastToABP_Saya (Components|SkeletalMesh|GetAnimInstance (Variables|Character|GetMesh))))
  (Variables|/Game/Characters/Saya/ABP_Saya.ABP_Saya_C|SetRotationHeadAlpha _asabp_saya alpha))

(event EventSetHeadRotation
  (params (rotator :type Rotator :default "0, 0, 0"))
  ;[1 1 1] 캐릭터 절차적 머리 회전
  (bind _asabp_saya (Utilities|Casting|CastToABP_Saya (Components|SkeletalMesh|GetAnimInstance (Variables|Character|GetMesh))))
  (Variables|/Game/Characters/Saya/ABP_Saya.ABP_Saya_C|SetHeadRotation _asabp_saya rotator))

(event EventSetInteractEndAnimation
  ;[1 1 1] 대화 애니메이션
  (bind _asabp_saya (Utilities|Casting|CastToABP_Saya (Components|SkeletalMesh|GetAnimInstance (Variables|Character|GetMesh))))
  (Variables|/Game/Characters/Saya/ABP_Saya.ABP_Saya_C|SetIsDone _asabp_saya true)
  (Variables|/Game/Characters/Saya/ABP_Saya.ABP_Saya_C|SetIsTalking _asabp_saya false)
  (Utilities|FlowControl|Delay 0.2)
  (Variables|/Game/Characters/Saya/ABP_Saya.ABP_Saya_C|SetIsDone _asabp_saya false))

(fn ConstructionScript)