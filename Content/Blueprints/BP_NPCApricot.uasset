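; BP_NPCApricot is the Apricot NPC Blueprint, exposing events that drive its procedural head rotation and talking animation.
; Each event casts the mesh's anim instance to ABP_Apricot and sets its variables directly, with separate events for head rotation and blend alpha.
; Interaction begin sets IsTalking, while interaction end clears it and pulses IsDone through a short Delay.
; BeginPlay, overlap, Tick and the construction script hold no logic.
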(event EventBeginPlay)

(event Collision|EventActorBeginOverlap
  (params (OtherActor :type Actor%20Object%20Reference)))

(event EventTick
  (params (DeltaSeconds :type Float%20%28single-precision%29)))

(event EventSetInteractBeginAnimation
  ;[1 1 1] 대화 애니메이션
  (bind _asabp_apricot (Utilities|Casting|CastToABP_Apricot (Components|SkeletalMesh|GetAnimInstance (Variables|Character|GetMesh))))
  (Variables|/Game/Characters/Apricot/ABP_Apricot.ABP_Apricot_C|SetIsTalking _asabp_apricot true))

(event EventSetHeadRotationAlpha
  (params (alpha :type Float%20%28single-precision%29))
  ;[1 1 1] 캐릭터 절차적 머리 회전
  (bind _asabp_apricot (Utilities|Casting|CastToABP_Apricot (Components|SkeletalMesh|GetAnimInstance (Variables|Character|GetMesh))))
  (Variables|/Game/Characters/Apricot/ABP_Apricot.ABP_Apricot_C|SetRotationHeadAlpha _asabp_apricot alpha))

(event EventSetHeadRotation
  (params (rotator :type Rotator :default "0, 0, 0"))
  ;[1 1 1] 캐릭터 절차적 머리 회전
  (bind _asabp_apricot (Utilities|Casting|CastToABP_Apricot (Components|SkeletalMesh|GetAnimInstance (Variables|Character|GetMesh))))
  (Variables|/Game/Characters/Apricot/ABP_Apricot.ABP_Apricot_C|SetHeadRotation _asabp_apricot rotator))

(event EventSetInteractEndAnimation
  ;[1 1 1] 대화 애니메이션
  (bind _asabp_apricot (Utilities|Casting|CastToABP_Apricot (Components|SkeletalMesh|GetAnimInstance (Variables|Character|GetMesh))))
  (Variables|/Game/Characters/Apricot/ABP_Apricot.ABP_Apricot_C|SetIsDone _asabp_apricot true)
  (Variables|/Game/Characters/Apricot/ABP_Apricot.ABP_Apricot_C|SetIsTalking _asabp_apricot false)
  (Utilities|FlowControl|Delay 0.2)
  (Variables|/Game/Characters/Apricot/ABP_Apricot.ABP_Apricot_C|SetIsDone _asabp_apricot false))

(fn ConstructionScript)