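; Phantom enemy character that detects the Link player character and attacks with a GAS melee ability.
; AI perception updates blackboard keys for sight, follow target and a Peace/Chase monster state, which Tick prints for debugging.
; A separate attack capsule's overlaps send a melee damage gameplay event through a DoOnce, but the call enabling its collision is unwired.
; Damage plays a hit montage, or at zero health sets IsDead and disables collision.
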(event OnComponentBeginOverlap(Capsule)
  (params (OverlappedComponent :type Primitive%20Component%20Object%20Reference) (OtherActor :type Actor%20Object%20Reference) (OtherComp :type Primitive%20Component%20Object%20Reference) (OtherBodyIndex :type Integer) (bFromSweep :type Boolean) (SweepResult :type Hit%20Result%20Structure%20%28by%20ref%29))
  (if (!= (Utilities|GetClass OtherActor) (Utilities|GetClass (Game|GetInstigator)))
    (Utilities|FlowControl|DoOnce false
      (:Completed
        (Ability|SendGameplayEventtoActor self "(TagName=\"Ability.Melee.Damage\")" (Utilities|Struct|MakeGameplayEventData "(TagName=\"\")" (Game|GetInstigator) OtherActor))))))

(event OnComponentEndOverlap(Capsule)
  (params (OverlappedComponent :type Primitive%20Component%20Object%20Reference) (OtherActor :type Actor%20Object%20Reference) (OtherComp :type Primitive%20Component%20Object%20Reference) (OtherBodyIndex :type Integer))
  (Utilities|FlowControl|Delay 0.2)
  (Utilities|FlowControl|DoOnce false) ; enters at Reset
)

(event OnTargetPerceptionUpdated(AIPerception)
  (params (Actor :type Actor%20Object%20Reference) (Stimulus :type AI%20Stimulus%20Structure))
  (bind _returnvalue (AI|GetBlackboard 0))
  (bind _asbp_link_character (Utilities|Casting|CastToBP_LinkCharacter Actor)
    (:then
      (Utilities|FlowControl|Sequence
        (:then_0
          (AI|Components|Blackboard|SetValueasBool _returnvalue (Utilities|Name|MakeLiteralName "CanSeePlayer") (.bSuccessfullySensed (Utilities|Struct|BreakAIStimulus Stimulus)))
          (bind _output_get (Variables|Default|SetMonsterState "Chase"))
          (AI|Components|Blackboard|SetValueasEnum (AI|GetBlackboard 0) (Utilities|Name|MakeLiteralName "MonsterState") _output_get))
        (:then_1
          (AI|Components|Blackboard|SetValueasObject _returnvalue (Utilities|Name|MakeLiteralName "TargetToFollow") _asbp_link_character))))
    (:CastFailed
      (AI|Components|Blackboard|SetValueasObject _returnvalue (Utilities|Name|MakeLiteralName "TargetToFollow") 0))))

(event EventBeginPlay
  (Collision|SetCollisionEnabled (Variables|Default|GetCapsule) "NoCollision")
  (bind _output_get (Variables|Default|SetMonsterState "Peace"))
  (AI|Components|Blackboard|SetValueasEnum (AI|GetBlackboard 0) (Utilities|Name|MakeLiteralName "MonsterState") _output_get))

(event EventTick
  (params (DeltaSeconds :type Float%20%28single-precision%29))
  (Development|PrintString (Utilities|String|ToString(Byte) (Class|BlackboardComponent|GetValueasEnum (AI|GetBlackboard 0) (Utilities|Name|MakeLiteralName "MonsterState"))) true true "(R=0.000000,G=0.660000,B=1.000000,A=1.000000)" 0.0))

(event EventOnAttacking
  (Abilities|TryActivateAbilitybyClass (Variables|Default|GetAbilitySystemComponent) "/Game/Abilities/Enemies/Phantom/GA_PhantomMelee.GA_PhantomMelee_C" true))

(event EventOnDamaged
  (params (DamageAmount :type Float%20%28single-precision%29) (HitInfo :type Hit%20Result%20Structure%20%28by%20ref%29) (DamageTags :type Gameplay%20Tag%20Container%20Structure%20%28by%20ref%29) (InstigatorCharacter :type Character%20Base%20Object%20Reference) (DamageCauser :type Actor%20Object%20Reference))
  (if (> (Class|CharacterBase|GetHealth) 0.0)
    (Animation|PlayAnimMontage "/Game/Monsters/Phantom/Animations/Dam_Montage.Dam_Montage" 1.0 "None")
    (else
      (Variables|Default|SetIsDead true)
      ;[1 1 1] 임시
      (Collision|SetCollisionEnabled (Variables|Default|GetCapsule) "NoCollision")
      (Collision|SetCollisionEnabled (Variables|Default|GetCapsuleComponent) "NoCollision"))))

(event EventEventBeginAttack)

(event EventEventEndAttack
  (Utilities|FlowControl|Delay 0.2)
  (Collision|SetCollisionEnabled (Variables|Default|GetCapsule) "NoCollision"))

(fn ConstructionScript)