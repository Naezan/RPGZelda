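; BP_TransitionLevel is a trigger actor that plays a short exit sequence and loads another level when the Link character overlaps it.
; It hides the RPG controller's HUD, unpossesses the character and gives it a default controller to AI-walk toward a random navigable point near its Destination component.
; As the move begins, the view blends to the actor and the camera fades out before the configured Level opens with Options.
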(event EventBeginPlay)

(event Collision|EventActorBeginOverlap
  (params (OtherActor :type Actor%20Object%20Reference))
  (bind _asbp_link_character (Utilities|Casting|CastToBP_LinkCharacter OtherActor))
  (bind _asbp_rpgplayer_controller (Utilities|Casting|CastToBP_RPGPlayerController (Game|GetPlayerController 0)))
  (Class|RPGPlayerController|ShowHUD _asbp_rpgplayer_controller false)
  (Pawn|UnPossess _asbp_rpgplayer_controller)
  (Pawn|SpawnDefaultController _asbp_link_character)
  (AI|AIMoveTo _asbp_link_character (.RandomLocation (Class|NavigationSystemV1|GetRandomPointinNavigableRadius (Transformation|GetWorldLocation (Variables|Default|GetDestination)) 5e+01 0 0)) 0 5.0 false
    (:then
      (Game|Player|SetViewTargetwithBlend (Game|GetPlayerController 0) self 1.0 "VTBlend_Linear" 0.0 false)
      (CameraFades|StartCameraFade :self (Game|GetPlayerCameraManager 0) :ToAlpha 1.0 :Duration 2.0 :bHoldWhenFinished true)
      (Utilities|FlowControl|Delay 2.0)
      (Game|OpenLevel(byObjectReference) (Variables|Default|GetLevel) true (Variables|Default|GetOptions)))))

(fn ConstructionScript)