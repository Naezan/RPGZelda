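; Player controller for a Zelda-style RPG that sets up the player's UI, weapons and save data.
; On BeginPlay it adds a drawing widget with cursor-enabled game-and-UI input, views the pawn, creates the Link character's weapons and builds an initially hidden HUD.
; Events toggle HUD visibility and refresh its icons when items change.
; InitSaveData loads through the game mode, recreates weapons, then saves.
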(event Custom|CreateHUD
  (Utilities|IsValid (Variables|Default|GetHUD)
    (:Is%20Valid
      _)
    (:Is%20Not%20Valid
      (bind _returnvalue (UserInterface|CreateWidget "/Game/UI/WBP_HUD.WBP_HUD_C" self))
      (bind _output_get (Variables|Default|SetHUD _returnvalue))
      (UserInterface|Viewport|AddtoViewport _output_get 0)
      (Class|IHUD|UpdateIcons(Message) (Variables|Default|GetHUD))))
  (Class|RPGPlayerController|ShowHUD false))

(event Custom|UpdateOnScreenIcon
  (Class|IHUD|UpdateIcons(Message) (Variables|Default|GetHUD)))

(event EventBeginPlay
  (bind _returnvalue (Pawn|GetControlledPawn))
  (|CallParentFunction)
  (Utilities|FlowControl|Sequence
    (:then_0
      (bind _returnvalue_2 (UserInterface|CreateWidget "/Game/UI/WBP_Drawing.WBP_Drawing_C" self))
      (UserInterface|Viewport|AddtoViewport _returnvalue_2 0)
      (bind _output_get (Variables|Default|SetDrawing _returnvalue_2))
      (Input|SetInputModeGameandUI self _output_get "DoNotLock" false)
      (Variables|Default|SetbShowMouseCursor true))
    (:then_1
      (Game|Player|SetViewTargetwithBlend _returnvalue 0.0 "VTBlend_Linear" 0.0 false)
      (bind _asbp_link_character (Utilities|Casting|CastToBP_LinkCharacter _returnvalue))
      (Variables|Default|SetPlayer%20Character _asbp_link_character))
    (:then_2
      (Default|CreateAllWeapons (Variables|Default|GetPlayer%20Character))
      (CallFunction|CreateHUD))))

(event EventGrantedItemChanged
  (Class|IHUD|UpdateIcons(Message) (Variables|Default|GetHUD)))

(event EventShowHUD
  (params (Visible :type Boolean))
  (bind _hud (Variables|Default|GetHUD))
  (Utilities|IsValid _hud
    (:Is%20Valid
      (Widget|SetVisibility _hud (select Visible "SelfHitTestInvisible" "Hidden")))))

(event EventPossess
  (params (PossessedPawn :type Pawn%20Object%20Reference))
  (Utilities|FlowControl|DoOnce false
    (:Completed
      (bind _asbp_link_character (Utilities|Casting|CastToBP_LinkCharacter PossessedPawn))
      (Variables|Default|SetPlayer%20Character _asbp_link_character))))

(event EventInitSaveData
  (bind _asbp_rpgzelda_game_mode (Utilities|Casting|CastToBP_RPGZeldaGameMode (Game|GetGameMode)))
  (Default|LoadGame _asbp_rpgzelda_game_mode self)
  (Default|CreateAllWeapons (Variables|Default|GetPlayer%20Character))
  (Default|SaveGame _asbp_rpgzelda_game_mode))

(fn ConstructionScript)