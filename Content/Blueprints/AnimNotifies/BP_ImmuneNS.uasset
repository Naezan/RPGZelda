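; Anim notify state that gives a character the immune gameplay effect for the span of an animation window.
; On begin it casts the mesh owner to CharacterBase and applies ImmuneEffect through that character's Ability System Component.
; On end it removes all stacks of that effect from the same component.
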(fn ReceivedNotifyBegin
  (params (MeshComp :type Skeletal%20Mesh%20Component%20Object%20Reference) (Animation :type Anim%20Sequence%20Base%20Object%20Reference) (TotalDuration :type Float%20%28single-precision%29))
  (bind _ascharacter_base (Utilities|Casting|CastToCharacterBase (Components|GetOwner MeshComp)))
  (GameplayEffects|ApplyGameplayEffectToSelf :self (Ability|GetAbilitySystemComponent _ascharacter_base) :GameplayEffectClass (Variables|Default|GetImmuneEffect))
  (return true))

(fn ReceivedNotifyEnd
  (params (MeshComp :type Skeletal%20Mesh%20Component%20Object%20Reference) (Animation :type Anim%20Sequence%20Base%20Object%20Reference))
  (bind _ascharacter_base (Utilities|Casting|CastToCharacterBase (Components|GetOwner MeshComp)))
  (GameplayEffects|RemoveActiveGameplayEffectbySourceEffect (Ability|GetAbilitySystemComponent _ascharacter_base) (Variables|Default|GetImmuneEffect) 0 -1)
  (return true))