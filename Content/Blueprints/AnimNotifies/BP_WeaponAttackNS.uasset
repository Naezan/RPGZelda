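; Anim notify state that marks the active attack window of the Link character's weapon during an attack animation.
; On begin and end it casts the mesh owner to BP_LinkCharacter and gets its current weapon as BP_Weapon.
; It then calls the weapon's begin or end attack event, leaving the attack logic itself to the weapon.
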(fn ReceivedNotifyBegin
  (params (MeshComp :type Skeletal%20Mesh%20Component%20Object%20Reference) (Animation :type Anim%20Sequence%20Base%20Object%20Reference) (TotalDuration :type Float%20%28single-precision%29))
  (bind _asbp_link_character (Utilities|Casting|CastToBP_LinkCharacter (Components|GetOwner MeshComp)))
  (Utilities|IsValid (Variables|/Script/RPGZelda.LinkCharacter|GetCurrentWeapon _asbp_link_character)
    (:Is%20Valid
      (bind _asbp_weapon (Utilities|Casting|CastToBP_Weapon (Variables|/Script/RPGZelda.LinkCharacter|GetCurrentWeapon _asbp_link_character)))
      (Default|EventBeginWeaponAttack _asbp_weapon)
      (return false))))

(fn ReceivedNotifyEnd
  (params (MeshComp :type Skeletal%20Mesh%20Component%20Object%20Reference) (Animation :type Anim%20Sequence%20Base%20Object%20Reference))
  (bind _asbp_link_character (Utilities|Casting|CastToBP_LinkCharacter (Components|GetOwner MeshComp)))
  (Utilities|IsValid (Variables|/Script/RPGZelda.LinkCharacter|GetCurrentWeapon _asbp_link_character)
    (:Is%20Valid
      (bind _asbp_weapon (Utilities|Casting|CastToBP_Weapon (Variables|/Script/RPGZelda.LinkCharacter|GetCurrentWeapon _asbp_link_character)))
      (Default|EventEndWeaponAttack _asbp_weapon) ; 충돌체
      (return false))))