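; Gameplay Ability for the player's sword melee attack that deals damage through GE_PlayerSwordMelee.
; On activation it commits, plays a montage, and listens for the Ability.Melee.Damage gameplay event.
; Each received event applies the damage effect to the event's target and prints a debug string.
; The ability ends when the montage completes, blends out, or is interrupted or cancelled, and OnEndAbility calls CallOnAbilityEnded.
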(event Ability|EventActivateAbility
  ;[1 1 1] 데미지 이벤트가 들어오면 데미지이펙트를 내가 아닌 대상에게 적용해라
  (Ability|CommitAbility)
  (|PlayMontageandWaitProxy "None" (Variables|Default|GetMontageToPlay) 1.0 "None" true 1.0 0.0
    (:then
      (bind _payload (Ability|Tasks|WaitGameplayEvent "(TagName=\"Ability.Melee.Damage\")" 0)
        (:EventReceived
          (GameplayEffects|ApplyGameplayEffectToTarget (Ability|TargetData|AbilityTargetDatafromActor (.Target (Utilities|Struct|BreakGameplayEventData _payload))) "/Game/Abilities/Player/Sword/GE_PlayerSwordMelee.GE_PlayerSwordMelee_C" 1 1)
          (Development|PrintString "PlayerMelee"))))
    (:OnCompleted
      (Ability|EndAbility :!label _label))
    (:OnBlendOut
      (goto _label))
    (:OnInterrupted
      (goto _label))
    (:OnCancelled
      (goto _label))))

(event Ability|EventOnEndAbility
  (params (bWasCancelled :type Boolean))
  (Default|CallOnAbilityEnded))